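; Wheeled-vehicle reinforcement learning agent that learns to steer along road tiles using the external MindMaker engine over SocketIO.
; Tick traces left and right distances, which are sent with yaw as observations.
; Each received action sets steering at constant throttle, adds a small reward and emits the next observation.
; Death-tagged overlaps penalize and reposition the car; the launch config loads a pretrained model, skipping the training count.
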(event `Delay for display`
  (bind _wheeledvehiclemovementcomponent4w (`self.WheeledVehicleMovementComponent4W`))
  ;[1 1 1] When displaying actions after training we divert from the normal recieve action function to this one so that a pause can be added as the agent moves between locations
  (`WheeledVehicleMovementComponent.SetThrottleInput` _wheeledvehiclemovementcomponent4w 0.5)
  (`WheeledVehicleMovementComponent.SetSteeringInput` _wheeledvehiclemovementcomponent4w (`self.Action`))
  (`self.MakeObservations`)
  (`self.CheckReward`)
  (setmembers `/Game/MindMaker/Examples/Assets/CartPole/MindMakerCustomStructCont` :`StructRef` (`self.MindMakerStructure`) :`reward` (`self.Reward`) :`observations` (`self.Observations`) :`done` (`self.done`))
  (`SocketIOClientComponent.Emit` (`self.SocketIOClient`) "sendobs" (`SIOJLibrary.Conv_StringToJsonValue` (`SIOJsonObject.EncodeJson` (`SIOJLibrary.StructToJsonObject` (`self.MindMakerStructure`)))) "/")
  (set `self.ExploreCounter` (+ (`self.ExploreCounter`) 1))
  (if (== (- (`self.ExploreCounter`) (`self.NumTrainingEpisodes`)) (`self.NumEvalEpisodes`))
    (`KismetSystemLibrary.PrintString` "Finished Evaluation")))

(event `self.SocketIOClient.OnConnected`
  (params (SessionId :type String) (bIsReconnection :type Boolean))
  ;[1 1 1] Launch MindMaker
  ;;[1 1 1] If not using the mindmaker launcher plugin, manually launch mindmaker.exe before begining play. This is located in the MindMakerEngine directory within the projects Content folder. NOTE uses SocketIO to communicate with mindmaker.exe so your OS or antivirus may ask for user permission to access network.
  ;;[1 1 1] recieve messages from MindMaker
  (`SocketIOClientComponent.BindEventToFunction` (`self.SocketIOClient`) "messages" "Messages" null "/" "USE_DEFAULT") ; bind event to a bp function
  (`SocketIOClientComponent.BindEventToFunction` (`self.SocketIOClient`) "recaction" "ReceiveAction" null "/" "USE_DEFAULT") ; bind event to a bp function
  (`SocketIOClientComponent.BindEventToFunction` (`self.SocketIOClient`) "sendobs" "SendObservations" null "/" "USE_DEFAULT") ; bind event to a bp function
  (`SocketIOClientComponent.Connect` (`self.SocketIOClient`) "http://localhost:3000" "socket.io" null null)
  (`self.LaunchMindMaker` "NewEnumerator8" (`self.NumTrainingEpisodes`) (`self.NumEvalEpisodes`) true false true false "car_test_01" "low=-1, high=1,shape=(1,)" "low=np.array([-10000,-10000,-10000]), high=np.array([10000,10000,-10000]),dtype=np.float32" true (`self.A2c Custom Params`) (struct) (struct) (`self.Dqn Custom Params`)))

(event `self.ReceiveBeginPlay`
  ;[1 1 1] Launch MindMaker
  ;;[1 1 1] To autolaunch the Mindmaker engine on event begin play, for instance in production use cases, requires the Mindmaker Launcher Plugin to be installed
  (`PlayerController.SetViewTargetWithBlend` (`GameplayStatics.GetPlayerController` 0) self 0.0 "VTBlend_Linear" 0.0 false)
  (`GameplayStatics.SetGlobalTimeDilation` 2.0)
  (`MindMakerBPLibrary.MindMakerWindows`)
  (`KismetSystemLibrary.PrintString` "MindMaker Launched")
  (`KismetSystemLibrary.PrintString` "Waiting for Connection from Learning Engine" true true (struct :`G` 0.66 :`B` 1.0 :`A` 1.0) 60.0))

(event `self.ReceiveTick`
  (params (DeltaSeconds :type "Float (single-precision)"))
  (bind _arrowright (`self.ArrowRight`))
  (bind _arrowleft (`self.ArrowLeft`))
  (bind _returnvalue (`SceneComponent.K2_GetComponentLocation` _arrowleft))
  (bind _returnvalue_2 (`SceneComponent.K2_GetComponentLocation` _arrowright))
  (`|ExecutionSequence`
    (:`then_0`
      (bind (_outhit _returnvalue_3) (`KismetSystemLibrary.LineTraceSingle` :`Start` _returnvalue :`End` (+ _returnvalue (* (`KismetMathLibrary.GetForwardVector` (`SceneComponent.K2_GetComponentRotation` _arrowleft)) 1000000.0)) :`TraceChannel` "TraceTypeQuery1" :`DrawDebugType` "ForOneFrame"))
      (if _returnvalue_3
        (set `self.DistanceLeft` (`.Distance` (`GameplayStatics.BreakHitResult` _outhit)))
        (else
          (set `self.DistanceLeft` 100000.0))))
    (:`then_1`
      (bind (_outhit_2 _returnvalue_4) (`KismetSystemLibrary.LineTraceSingle` :`Start` _returnvalue_2 :`End` (+ _returnvalue_2 (* (`KismetMathLibrary.GetForwardVector` (`SceneComponent.K2_GetComponentRotation` _arrowright)) 1000000.0)) :`TraceChannel` "TraceTypeQuery1" :`DrawDebugType` "ForOneFrame"))
      (if _returnvalue_4
        (set `self.DistanceRight` (`.Distance` (`GameplayStatics.BreakHitResult` _outhit_2)))
        (else
          (set `self.DistanceLeft` 100000.0))))))

(event `self.SkeletalMesh.OnComponentBeginOverlap`
  (params (OverlappedComponent :type "PrimitiveComponent Object Reference") (OtherActor :type "Actor Object Reference") (OtherComp :type "PrimitiveComponent Object Reference") (OtherBodyIndex :type Integer) (bFromSweep :type Boolean) (SweepResult :type "HitResult Structure (by ref)"))
  (bind (_returnvalue_x _returnvalue_y) (`KismetMathLibrary.BreakVector` (`SceneComponent.K2_GetComponentLocation` (`self.SkeletalMesh`))))
  (cast `/Game/Blueprints/RoadTile` OtherActor)
  (if (`ActorComponent.ComponentHasTag` OtherComp "Death")
    (`self.AddReward` -1.0)
    (`self.K2_SetActorLocation` (`KismetMathLibrary.MakeVector` -10.948097 _returnvalue_y 24.891777) true true)
    (`self.K2_SetActorRotation` (struct :`Yaw` -90.0) true)))

(fn `AddReward`
  (params (Amount :type "Float (double-precision)"))
  (set `self.Reward` (+ (`self.Reward`) Amount)))

(fn `CheckReward`
  (set `self.Reward` (+ (`self.Reward`) 0.1)))

(fn `DisplayAgentAction`
  (bind _wheeledvehiclemovementcomponent4w (`self.WheeledVehicleMovementComponent4W`))
  (`WheeledVehicleMovementComponent.SetThrottleInput` _wheeledvehiclemovementcomponent4w 0.5)
  (`WheeledVehicleMovementComponent.SetSteeringInput` _wheeledvehiclemovementcomponent4w (`self.Action`)))

(fn `LaunchMindMaker`
  (params (`RL Algorithm` :type "/Game/MindMaker/Examples/Assets/MatchToSample/LearningAlgorithms Enum" :default "NewEnumerator0") (NumTrainEp :type Integer) (NumEvalEp :type Integer) (ContinousActionSpace :type Boolean) (DiscreteActionSpace :type Boolean) (LoadPreTrainedModel :type Boolean) (SaveModelAfterTraining :type Boolean) (`Save/LoadModelName` :type String) (ActionSpaceShape :type String) (ObservationSpaceShape :type String) (UseCustomParams :type Boolean) (A2cCustomParams :type "/Game/MindMaker/Examples/Assets/MatchToSample/A2cCustomParameters Structure") (AcerCustomParams :type "/Game/MindMaker/Examples/Assets/MatchToSample/AcerCustomParameters Structure") (AcktrCustomParams :type "/Game/MindMaker/Examples/Assets/MatchToSample/AcktrCustomParameters Structure") (DqnCustomParams :type "/Game/MindMaker/Examples/Assets/MatchToSample/DqnCustomParameters Structure") (Ppo2CustomParams :type "/Game/MindMaker/Examples/Assets/MatchToSample/PPO2CustomParameters Structure") (SacCustomParams :type "/Game/MindMaker/Examples/Assets/MatchToSample/SacCustomParameters Structure") (Td3CustomParams :type "/Game/MindMaker/Examples/Assets/MatchToSample/Td3CustomParameters Structure"))
  ;[1 1 1] Set members of our custom structure used for storing variables and pass them to neural network
  (setmembers `/Game/MindMaker/Examples/Assets/MatchToSample/MindMakerCustomStruct` :`StructRef` (`self.ExampleStruct`) :`reward` (`self.Reward`) :`observations` (`self.Observations`) :`trainepisodes` NumTrainEp :`evalepisodes` NumEvalEp :`maxactions` (`self.MaxActions`) :`loadmodel` (`KismetStringLibrary.Conv_BoolToString` LoadPreTrainedModel) :`savemodel` (`KismetStringLibrary.Conv_BoolToString` SaveModelAfterTraining) :`algselected` `RL Algorithm` :`customparams` (`KismetStringLibrary.Conv_BoolToString` UseCustomParams) :`a2cparams` A2cCustomParams :`acerparams` AcerCustomParams :`acktrparams` AcktrCustomParams :`dqnparams` DqnCustomParams :`ddpgparams` (struct :`policy` "NewEnumerator17" :`gamma` 0.99 :`verbose` 1 :`_init_setup_model` "True" :`full_tensorboard_log` "False" :`n_cpu_tf_sess` "1" :`layers` "[64, 64]" :`buffer_size` "50000" :`nb_train_steps` 50 :`nb_rollout_steps` 100 :`nb_eval_steps` 100 :`normalize_observations` "False" :`tau` 0.001 :`param_noise_adaption_interval` 50 :`normalize_returns` "False" :`enable_popart` "False" :`observation_range` "(-5.0, 5.0)" :`critic_l2_reg` "0.0" :`actor_lr` 0.0001 :`critic_lr` 0.001 :`reward_scale` 1.0 :`render` "False" :`render_eval` "False" :`random_exploration` "0.0" :`act_func` "NewEnumerator3") :`ppo1params` (struct :`policy` "NewEnumerator3" :`gamma` 0.99 :`verbose` 1 :`_init_setup_model` "True" :`full_tensorboard_log` "False" :`n_cpu_tf_sess` "1" :`layers` "[64, 64]" :`timesteps_per_actorbatch` 256 :`clip_param` 0.2 :`entcoeff` 0.01 :`optim_epochs` 4.0 :`optim_stepsize` 0.001 :`optim_batchsize` 64 :`lam` 0.95 :`adam_epsilon` 5e-05 :`schedule` "linear" :`act_func` "NewEnumerator3") :`ppo2params` Ppo2CustomParams :`sacparams` SacCustomParams :`td3params` Td3CustomParams :`trpoparams` (struct :`policy` "NewEnumerator3" :`gamma` 0.99 :`verbose` 1 :`_init_setup_model` "True" :`full_tensorboard_log` "False" :`n_cpu_tf_sess` "1" :`layers` "[64, 64]" :`entcoeff` 0.01 :`lam` 0.98 :`timesteps_per_batch` 1024 :`max_kl` 0.01 :`cg_iters` 10 :`cg_damping` 0.01 :`vf_stepsize` 0.0003 :`vf_iters` 3 :`act_func` "NewEnumerator3") :`modelname` `Save/LoadModelName` :`actionspace` ActionSpaceShape :`observationspace` ObservationSpaceShape :`conactionspace` ContinousActionSpace :`disactionspace` DiscreteActionSpace :`done` false)
  (if LoadPreTrainedModel
    (set `self.ExploreCounter` (`self.NumTrainingEpisodes`)))
  (`SocketIOClientComponent.Emit` (`self.SocketIOClient`) "launchmindmaker" (`SIOJLibrary.Conv_StringToJsonValue` (`SIOJsonObject.EncodeJson` (`SIOJLibrary.StructToJsonObject` (`self.ExampleStruct`)))) "/"))

(fn `MakeObservations`
  (bind (_returnvalue_roll _returnvalue_pitch _returnvalue_yaw) (`KismetMathLibrary.BreakRotator` (`SceneComponent.K2_GetComponentRotation` (`self.SkeletalMesh`))))
  ;[1 1 1] Enter observation values into array seperated by commas
  (set `self.Observations` (`KismetStringLibrary.Concat_StrStr` "[" (`KismetStringLibrary.Conv_DoubleToString` (`self.DistanceLeft`)) "," (`KismetStringLibrary.Conv_DoubleToString` (`self.DistanceRight`)) "," (`KismetStringLibrary.Conv_DoubleToString` _returnvalue_yaw) "]")))

(fn `Messages`
  (params (Message :type "SIOJsonValue Object Reference"))
  (bind _returnvalue (`SIOJsonValue.AsString` Message))
  ;[1 1 1] Display Messages From MindMaker.exe
  (`KismetSystemLibrary.PrintString` _returnvalue)
  (if (`KismetStringLibrary.EqualEqual_StrStr` _returnvalue "Training complete")
    (set `self.TrainingComplete` true)
    (elif (`KismetStringLibrary.EqualEqual_StrStr` _returnvalue "Evaluation Complete")
      (`KismetSystemLibrary.PrintString` "Quiting Game")
      (`KismetSystemLibrary.QuitGame` null "Quit"))))

(fn `ReceiveAction`
  (params (Message :type "SIOJsonValue Object Reference"))
  ;[1 1 1] This recieves results from the neural network and updates the environment
  (set `self.Action` (`KismetStringLibrary.Conv_StringToDouble` (`KismetStringLibrary.Replace` (`|GetArrayItem` (`KismetStringLibrary.ParseIntoArray` (`SIOJsonValue.AsString` Message))) "[")))
  (set `self.ActionRecieved` true)
  (if (< (`self.ExploreCounter`) (`self.NumTrainingEpisodes`))
    (`self.Delay for display`)
    (else
      (`self.DisplayAgentAction`)
      (`self.Delay for display`))))

(fn `UserConstructionScript`)